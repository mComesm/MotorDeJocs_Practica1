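; AI controller for BP_AI patrol characters that runs the AI_BT behavior tree.
; On BeginPlay it caches the controlled pawn and seeds the blackboard with its patrol path looping flag and wait time, plus a forward direction.
; AI perception updates set CanSeePlayer whenever a ThirdPersonCharacter is sensed or lost.
; A node that would store the stimulus location as TargetLocation is left unconnected.
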(event OnTargetPerceptionUpdated(AIPerception)
  (params (Actor :type Actor%20Object%20Reference) (Stimulus :type AI%20Stimulus%20Structure))
  (Utilities|Casting|CastToThirdPersonCharacter Actor)
  (AI|Components|Blackboard|SetValueasBool (AI|GetBlackboard 0) (Utilities|Name|MakeLiteralName "CanSeePlayer") (.bSuccessfullySensed (Utilities|Struct|BreakAIStimulus Stimulus))))

(event EventBeginPlay
  (bind _returnvalue (AI|GetBlackboard 0))
  (AI|RunBehaviorTree "/Game/AI/AI_BT.AI_BT")
  (bind _asbp_ai (Utilities|Casting|CastToBP_AI (Pawn|GetControlledPawn)))
  (bind _output_get (Variables|Default|SetMyPawn _asbp_ai))
  (AI|Components|Blackboard|SetValueasBool _returnvalue (Utilities|Name|MakeLiteralName "PathLooping") (Variables|/Game/AI/BP_PatrolPath.BP_PatrolPath_C|GetisLooping (Variables|/Game/AI/BP_AI.BP_AI_C|GetPatrolPath _output_get)))
  (Class|BlackboardComponent|SetValueasInt _returnvalue (Utilities|Name|MakeLiteralName "Direction") 1)
  (AI|Components|Blackboard|SetValueasFloat _returnvalue (Utilities|Name|MakeLiteralName "WaitTime") (Variables|/Game/AI/BP_PatrolPath.BP_PatrolPath_C|GetWaitTime (Variables|/Game/AI/BP_AI.BP_AI_C|GetPatrolPath (Variables|Default|GetMyPawn)))))

(fn ConstructionScript)