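; BP_AI is an AI character with a floating health bar, a slow walk speed and a melee attack.
; Tick yaws the health bar toward the player, and AnyDamage sets its progress from Health minus Damage without storing the reduced Health.
; A MeleeAttack event plays an attack montage and prints a debug string.
; The construction script tints the body dark through a dynamic material instance.
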(event EventBeginPlay
  (Variables|/Script/Engine.CharacterMovementComponent|SetMaxWalkSpeed (Variables|Character|GetCharacterMovement) 2e+02))

(event Collision|EventActorBeginOverlap
  (params (OtherActor :type Actor%20Object%20Reference)))

(event EventTick
  (params (DeltaSeconds :type Float%20%28single-precision%29))
  ;[1 1 1] Health bar Rotation
  (Transformation|SetWorldRotation (Variables|Default|GetHealthBar) (Math|Rotator|MakeRotator 0.0 0.0 (.Yaw (Math|Rotator|BreakRotator (Math|Rotator|FindLookatRotation (Transformation|GetWorldLocation (Variables|Default|GetHealthBar)) (Transformation|GetActorLocation (Game|GetPlayerCharacter 0)))))) false false))

(event Game|Damage|EventAnyDamage
  (params (Damage :type Float%20%28single-precision%29) (DamageType :type Damage%20Type%20Object%20Reference) (InstigatedBy :type Controller%20Object%20Reference) (DamageCauser :type Actor%20Object%20Reference))
  (bind _asbp_ai_health (Utilities|Casting|CastToBP_AI_Health (UserInterface|GetUserWidgetObject (Variables|Default|GetHealthBar))))
  (Progress|SetPercent (Variables|/Game/HUD/BP_AI_Health.BP_AI_Health_C|GetProgressBar_55 _asbp_ai_health) (/ (- (Variables|Default|GetHealth) Damage) 1e+02)))

(event EventMeleeAttack
  (Animation|Montage|PlayMontage (Variables|Character|GetMesh) "/Game/AI/Attack_PrimaryA_Montage.Attack_PrimaryA_Montage"
    (:then
      (Development|PrintString "Attack"))))

(fn ConstructionScript
  (bind _returnvalue (Rendering|Material|CreateDynamicMaterialInstance "/Game/Mannequin/Character/Materials/M_UE4Man_Body.M_UE4Man_Body" "None" :!class /Script/Engine.KismetMaterialLibrary))
  (Rendering|Material|SetVectorParameterValue _returnvalue "BodyColor" "(R=0.010417,G=0.010378,B=0.010263,A=1.000000)" :!class /Script/Engine.MaterialInstanceDynamic)
  (Rendering|Material|SetMaterial (Variables|Character|GetMesh) 0 _returnvalue))