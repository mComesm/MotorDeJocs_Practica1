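; Child Blueprint of LightBulb that acts as a color-matching bulb with a target color and a completion flag.
; An actor overlap runs the parent handler, then calls ChangeLight.
; Every tick it compares the PointLight color to GoodColor with a small tolerance and sets Done to true on a match, with no reset here.
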(event EventBeginPlay
  (|CallParentFunction) ; This node is disabled and will not be called.\nDrag off pins to build functionality.
)

(event Collision|EventActorBeginOverlap
  (params (OtherActor :type Actor%20Object%20Reference))
  (|CallParentFunction OtherActor)
  (CallFunction|ChangeLight))

(event EventTick
  (params (DeltaSeconds :type Float%20%28single-precision%29))
  (bind _pointlight (Variables|Default|GetPointLight))
  (bind _returnvalue (Rendering|Components|Light|GetLightColor _pointlight))
  (|CallParentFunction DeltaSeconds)
  (if (Math|Vector|Equal(Vector) (Math|Vector|MakeVector (.r _returnvalue) (.g _returnvalue) (.b _returnvalue)) (Variables|Default|GetgoodColor) 0.0001)
    (Variables|Default|Setdone true)))

(fn ConstructionScript
  (|CallParentFunction))