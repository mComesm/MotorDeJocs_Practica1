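; LightBulb is a Blueprint light bulb object whose point light color can be cycled through a list of colors.
; Each ChangeLight call advances an index through the AllColors array, wraps to the first entry past the end, and applies that vector as RGB with full alpha.
; The event graph and construction script do nothing, and nothing in the Blueprint calls ChangeLight.
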(event EventBeginPlay)

(event Collision|EventActorBeginOverlap
  (params (OtherActor :type Actor%20Object%20Reference)))

(event EventTick
  (params (DeltaSeconds :type Float%20%28single-precision%29)))

(fn ConstructionScript)

(fn ChangeLight
  (bind _output_get (Variables|Default|Setindex (+ (Variables|Default|Getindex) 1)))
  (if (> _output_get (Utilities|Array|LastIndex (Variables|Default|GetallColors)))
    (bind _output_get_2 (Variables|Default|Setindex 0))
    (Rendering|Components|Light|SetLightColor (Variables|Default|GetPointLight) (Utilities|Struct|MakeLinearColor (.x (Utilities|Array|Get(acopy) (Variables|Default|GetallColors) _output_get_2)) (.y (Utilities|Array|Get(acopy) (Variables|Default|GetallColors) _output_get_2)) (.z (Utilities|Array|Get(acopy) (Variables|Default|GetallColors) _output_get_2)) 1.0) true)
    (else
      (Rendering|Components|Light|SetLightColor (Variables|Default|GetPointLight) (Utilities|Struct|MakeLinearColor (.x (Utilities|Array|Get(acopy) (Variables|Default|GetallColors) (Variables|Default|Getindex))) (.y (Utilities|Array|Get(acopy) (Variables|Default|GetallColors) (Variables|Default|Getindex))) (.z (Utilities|Array|Get(acopy) (Variables|Default|GetallColors) (Variables|Default|Getindex))) 1.0) true))))