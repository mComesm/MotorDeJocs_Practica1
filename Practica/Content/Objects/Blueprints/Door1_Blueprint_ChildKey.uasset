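; A key-locked child variant of the Door1 Blueprint that opens only for a player carrying a key.
; On BeginPlay it runs the parent logic, then disables opening and closing.
; When a ThirdPersonCharacter with at least one key enters the Box and Done is false, it calls SetKey(-1), enables CanOpen and calls the parent's ActorBeginOverlap.
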(event OnComponentBeginOverlap(Box)
  (params (OverlappedComponent :type Primitive%20Component%20Object%20Reference) (OtherActor :type Actor%20Object%20Reference) (OtherComp :type Primitive%20Component%20Object%20Reference) (OtherBodyIndex :type Integer) (bFromSweep :type Boolean) (SweepResult :type Hit%20Result%20Structure%20%28by%20ref%29))
  (if (not (Variables|Default|Getdone))
    (bind _asthird_person_character (Utilities|Casting|CastToThirdPersonCharacter OtherActor))
    (if (>= (Variables|/Game/ThirdPersonBP/Blueprints/ThirdPersonCharacter.ThirdPersonCharacter_C|Getkeys _asthird_person_character) 1)
      (Default|SetKey _asthird_person_character -1)
      (Variables|Default|SetcanOpen true)
      (|CallParentFunction 0))))

(event EventBeginPlay
  (|CallParentFunction)
  (Variables|Default|SetcanOpen false)
  (Variables|Default|SetcanClose false))

(event Collision|EventActorBeginOverlap
  (params (OtherActor :type Actor%20Object%20Reference))
  (|CallParentFunction OtherActor) ; This node is disabled and will not be called.\nDrag off pins to build functionality.
)

(event EventTick
  (params (DeltaSeconds :type Float%20%28single-precision%29))
  (|CallParentFunction DeltaSeconds) ; This node is disabled and will not be called.\nDrag off pins to build functionality.
)

(fn ConstructionScript
  (|CallParentFunction))