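; A platform actor that dissolves and stops being solid after something overlaps its trigger box.
; Box overlap creates a dynamic material on the mesh and plays a timeline that drives its DissolutionValue parameter.
; In parallel, a short delay disables the actor's collision; nothing connected restores it or destroys the actor.
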(event OnComponentBeginOverlap(Box)
  (params (OverlappedComponent :type Primitive%20Component%20Object%20Reference) (OtherActor :type Actor%20Object%20Reference) (OtherComp :type Primitive%20Component%20Object%20Reference) (OtherBodyIndex :type Integer) (bFromSweep :type Boolean) (SweepResult :type Hit%20Result%20Structure%20%28by%20ref%29))
  (Utilities|FlowControl|Sequence
    (:then_0
      (bind _returnvalue (Rendering|Material|CreateDynamicMaterialInstance (Variables|Default|GetStaticMesh) 0 0 "None" :!class /Script/Engine.PrimitiveComponent))
      (bind _newtrack_0 (Timeline|Timeline_0 Play)
        (:Update
          (Rendering|Material|SetScalarParameterValue _returnvalue "DissolutionValue" _newtrack_0 :!class /Script/Engine.MaterialInstanceDynamic))))
    (:then_1
      (Utilities|FlowControl|Delay 1.0)
      (Collision|SetActorEnableCollision false))))

(event OnComponentEndOverlap(StaticMesh)
  (params (OverlappedComponent :type Primitive%20Component%20Object%20Reference) (OtherActor :type Actor%20Object%20Reference) (OtherComp :type Primitive%20Component%20Object%20Reference) (OtherBodyIndex :type Integer)))

(event EventBeginPlay)

(event Collision|EventActorBeginOverlap
  (params (OtherActor :type Actor%20Object%20Reference)))

(event EventTick
  (params (DeltaSeconds :type Float%20%28single-precision%29)))

(fn ConstructionScript)