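; Sliding door actor that opens on overlap and can close again when an overlap ends.
; BeginPlay stores the start location, and the Door timeline adds its Movement offset to it to move the whole actor.
; Actor or Box begin overlap plays the timeline if CanOpen, and Box end overlap reverses it if CanClose.
; Box overlaps skip the player cast, and the actor overlap casts player pawn 0, not the overlapping actor.
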(event OnComponentBeginOverlap(Box)
  (params (OverlappedComponent :type Primitive%20Component%20Object%20Reference) (OtherActor :type Actor%20Object%20Reference) (OtherComp :type Primitive%20Component%20Object%20Reference) (OtherBodyIndex :type Integer) (bFromSweep :type Boolean) (SweepResult :type Hit%20Result%20Structure%20%28by%20ref%29))
  (if (Variables|Default|GetcanOpen)
    (Variables|Default|Setdone true)
    (bind _movement (Timeline|Door Play)
      (:Update
        (Transformation|SetActorLocation (+ _movement (Variables|Default|GetinitPos)) false false)))))

(event OnComponentEndOverlap(Box)
  (params (OverlappedComponent :type Primitive%20Component%20Object%20Reference) (OtherActor :type Actor%20Object%20Reference) (OtherComp :type Primitive%20Component%20Object%20Reference) (OtherBodyIndex :type Integer))
  (if (Variables|Default|GetcanClose)
    (bind _movement (Timeline|Door Reverse)
      (:Update
        (Transformation|SetActorLocation (+ _movement (Variables|Default|GetinitPos)) false false)))))

(event EventBeginPlay
  (Variables|Default|SetinitPos (Transformation|GetActorLocation)))

(event Collision|EventActorBeginOverlap
  (params (OtherActor :type Actor%20Object%20Reference))
  ;[1 0.315 0.4148] Com castejo al jugador?
  (Utilities|Casting|CastToPlayerCharacter (Game|Player|GetPlayerPawn 0))
  (if (Variables|Default|GetcanOpen)
    (Variables|Default|Setdone true)
    (bind _movement (Timeline|Door Play)
      (:Update
        (Transformation|SetActorLocation (+ _movement (Variables|Default|GetinitPos)) false false)))))

(event EventTick
  (params (DeltaSeconds :type Float%20%28single-precision%29)))

(fn ConstructionScript)