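; BP_SaveGame is a save game object that holds test bool, int, float and transform values and handles its own slot saving and loading.
; SaveObject writes itself to a named slot synchronously, and an async save node sits unused in the event graph.
; LoadObject checks the slot and casts the loaded save, but assigns default values rather than loaded ones, or prints that none exists.
; PrintValues prints all four values.
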(fn SaveObject
  (params (SlotName :type String) (UserIndex :type Integer))
  (bind _returnvalue (SaveGame|SaveGametoSlot self SlotName UserIndex))
  (return _returnvalue))

(fn LoadObject
  (params (SlotName :type String) (UserIndex :type Integer))
  (bind _returnvalue (SaveGame|DoesSaveGameExist SlotName UserIndex))
  (if _returnvalue
    (bind _returnvalue_2 (SaveGame|LoadGamefromSlot SlotName UserIndex))
    (Utilities|Casting|CastToSaveGame _returnvalue_2)
    (Utilities|FlowControl|Sequence
      (:then_0
        (Variables|Default|SetMyBool false))
      (:then_1
        (Variables|Default|SetMyInt 0))
      (:then_2
        (Variables|Default|SetMyFloat 0.0))
      (:then_3
        (Variables|Default|SetMyTransform "")))
    (else
      (Development|PrintString 0 "No Saved Data Available"))))

(fn PrintValues
  (Development|PrintString 0 (Utilities|String|Append "My Bool: " (Utilities|String|ToString(Boolean) (Variables|Default|GetMyBool)) "My Int: " (Utilities|String|ToString(Integer) (Variables|Default|GetMyInt)) "My Float: " (Utilities|String|ToString(Float) (Variables|Default|GetMyFloat)) "My Transform: " (Utilities|String|ToString(Transform) (Variables|Default|GetMyTransform)))))